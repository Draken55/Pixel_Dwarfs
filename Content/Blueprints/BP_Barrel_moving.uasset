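; BP_Barrel_moving is a barrel actor that detects hits from the hero and reports whether the hero is holding an object.
; The Cube's hit event casts the other actor to BP_Hero_1, reads Isholdingobject and prints a debug message for either state.
; Disconnected node chains hold experiments that toggle collision or ignore the Pawn channel, none of which run.
; Tick and the construction script are empty.
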(event `self.ReceiveTick`
  (params (DeltaSeconds :type "Float (single-precision)")))

(event `self.Cube.OnComponentHit`
  (params (HitComponent :type "PrimitiveComponent Object Reference") (OtherActor :type "Actor Object Reference") (OtherComp :type "PrimitiveComponent Object Reference") (NormalImpulse :type "Vector Structure") (Hit :type "HitResult Structure (by ref)"))
  (bind _asbp_hero_1 (cast `/Game/Blueprints/Heros/BP_Hero_1` OtherActor))
  (if (`/Game/Blueprints/Heros/BP_Hero_1.isholdingobject` _asbp_hero_1)
    (`KismetSystemLibrary.PrintString` "IM HIT")
    (else
      (`KismetSystemLibrary.PrintString` "FAIL HIT"))))

(fn `UserConstructionScript`)