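; Timed moving platform that travels out and back when the player character steps onto it.
; A Box overlap by BP_Hero_1 moves the Cube to MoveTo with MoveComponentTo, waits for Timer, then moves it to MoveFrom.
; Other overlapping actors only print a debug message, and the end-overlap event is empty.
; Timeline-driven motion, OppositeRock direction switching and CharacterOver reset logic are mostly disconnected leftovers.
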(event `self.Box.OnComponentBeginOverlap`
  (params (OverlappedComponent :type "PrimitiveComponent Object Reference") (OtherActor :type "Actor Object Reference") (OtherComp :type "PrimitiveComponent Object Reference") (OtherBodyIndex :type Integer) (bFromSweep :type Boolean) (SweepResult :type "HitResult Structure (by ref)"))
  (cast `/Game/Blueprints/Heros/BP_Hero_1` OtherActor
    (:`then`
      (set `self.Character_over` true)
      (if (`self.Character_over`)
        (`KismetSystemLibrary.PrintString` "I AM TRUE")
        (`KismetSystemLibrary.MoveComponentTo` (`self.Cube`) (`self.Move_to`))
        (`KismetSystemLibrary.Delay` (`self.Timer`))
        (`KismetSystemLibrary.MoveComponentTo` (`self.Cube`) (`self.Move_from`))))
    (:`CastFailed`
      (`KismetSystemLibrary.PrintString` "CANT MOVE"))))

(event `self.Box.OnComponentEndOverlap`
  (params (OverlappedComponent :type "PrimitiveComponent Object Reference") (OtherActor :type "Actor Object Reference") (OtherComp :type "PrimitiveComponent Object Reference") (OtherBodyIndex :type Integer)))

(event `self.ReceiveActorBeginOverlap`
  (params (OtherActor :type "Actor Object Reference")))

(event `self.ReceiveActorEndOverlap`
  (params (OtherActor :type "Actor Object Reference")))

(event `self.ReceiveBeginPlay`)

(event `CustomEvent`
  (`|ExecutionSequence`
    (:`then_0`
      (if (`self.OppositeRock`)
        (bind (_direction _platform_motion) (`Timeline|Timeline_0` :!via `SetNewTime`))))))

(fn `UserConstructionScript`)