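; Paper2D side-scrolling player character (will-o'-the-wisp) that walks, sprints, jumps and can grab and throw physics objects.
; Enhanced Input drives single-axis movement, flipbook swaps and sprite flipping, with a delay loop polling vertical velocity to detect landing.
; Pickup line-traces from VectorSphere and grabs light simulating bodies with a PhysicsHandle, which follows HeldObjectLocation on Tick; pressing again releases and applies a throw impulse.
; Debug prints and some unreachable dash logic remain.
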(event `self.ReceiveBeginPlay`
  (set `CharacterMovementComponent.MaxWalkSpeed` 128.0 (`self.CharacterMovement`))
  (`KismetSystemLibrary.PrintString` "SPEED SET")
  (bind _asbp_player_controller (cast `/Game/Blueprints/BP_Player_Controller` (`self.GetController`))
    (:`then`
      (`EnhancedInputSubsystemInterface.AddMappingContext` (pcsubsystem `EnhancedInputLocalPlayerSubsystem` _asbp_player_controller) "/Game/Blueprints/IMC_Default.IMC_Default" 0 (struct))
      (`KismetSystemLibrary.PrintString` "Player1 Loaded"))
    (:`CastFailed`
      (`KismetSystemLibrary.PrintString` "FAIL LOAD"))))

(event `EnhancedInput|/Game/Blueprints/IA_Movement`
  (params (ActionValue :type "Float (double-precision)") (ElapsedSeconds :type "Float (double-precision)") (TriggeredSeconds :type "Float (double-precision)") (InputAction :type "InputAction Object Reference" :default "/Game/Blueprints/IA_Movement.IA_Movement"))
  (:`Triggered`
    (if (not (`self.is_jumping`))
      (`self.AddMovementInput` (`self.GetActorForwardVector`) ActionValue)
      (`PaperFlipbookComponent.SetFlipbook` (`self.Sprite`) "/Game/Assets/FP_Willo_wisp_walking1.FP_Willo_wisp_walking1")
      (if (> ActionValue 0.0)
        (`SceneComponent.K2_SetWorldRotation` :`self` (`self.Sprite`))
        (`SceneComponent.K2_SetWorldRotation` :`self` (`self.Vector_Sphere`))
        (else
          (`SceneComponent.K2_SetWorldRotation` (`self.Sprite`) (struct :`Yaw` -180.0) false false)
          (`SceneComponent.K2_SetWorldRotation` (`self.Vector_Sphere`) (struct :`Yaw` -180.0) false false)))))
  (:`Completed`
    (if (not (`self.is_jumping`))
      (`PaperFlipbookComponent.SetFlipbook` (`self.Sprite`) "/Game/Assets/FP_Willo_wisp_idle1.FP_Willo_wisp_idle1"))))

(event `EnhancedInput|/Game/Blueprints/IA_Jump`
  (params (ActionValue :type "Float (double-precision)") (ElapsedSeconds :type "Float (double-precision)") (TriggeredSeconds :type "Float (double-precision)") (InputAction :type "InputAction Object Reference" :default "/Game/Blueprints/IA_Jump.IA_Jump"))
  (bind _sprite (`self.Sprite`))
  (:`Triggered`
    (if (not (`self.is_jumping`))
      (set `self.is_jumping` true)
      (`self.Jump`)
      (`PaperFlipbookComponent.SetLooping` _sprite false)
      (`PaperFlipbookComponent.SetFlipbook` _sprite "/Game/Assets/FP_Willo_wisp_jump1.FP_Willo_wisp_jump1")
      (`KismetSystemLibrary.Delay` 0.1)
      (if (== (.z (`self.GetVelocity`)) 0.0) :!label _label
        (`PaperFlipbookComponent.SetLooping` _sprite true)
        (`PaperFlipbookComponent.Play` _sprite)
        (`PaperFlipbookComponent.SetFlipbook` _sprite "/Game/Assets/FP_Willo_wisp_idle1.FP_Willo_wisp_idle1")
        (set `self.is_jumping` false)
        (else
          (`KismetSystemLibrary.Delay` 0.2)
          (goto _label))))))

(event `InputAction|Grab`
  (params (Key :type "Key Structure")))

(event `EnhancedInput|/Game/Blueprints/IA_Sprint`
  (params (ActionValue :type "Float (double-precision)") (ElapsedSeconds :type "Float (double-precision)") (TriggeredSeconds :type "Float (double-precision)") (InputAction :type "InputAction Object Reference" :default "/Game/Blueprints/IA_Sprint.IA_Sprint"))
  (bind _charactermovement (`self.CharacterMovement`))
  ;[1 1 1] Run
  (:`Triggered`
    (if true
      (set `CharacterMovementComponent.MaxWalkSpeed` 300.0 _charactermovement)
      (`KismetSystemLibrary.PrintString` "RUN")))
  (:`Canceled`
    (set `CharacterMovementComponent.MaxWalkSpeed` 128.0 _charactermovement :!label _label_2)
    (`KismetSystemLibrary.PrintString` "walk"))
  (:`Completed`
    (goto _label_2)))

(event `Pickup`
  (bind _vector_sphere (`self.Vector_Sphere`))
  (bind _returnvalue (`SceneComponent.K2_GetComponentLocation` _vector_sphere))
  ;[1 1 1] Pick
  (bind (_outhit _returnvalue_2) (`KismetSystemLibrary.LineTraceSingle` :`Start` _returnvalue :`End` (+ _returnvalue (* (`SceneComponent.GetForwardVector` _vector_sphere) (10.0 0.0 0.0))) :`TraceChannel` "TraceTypeQuery2" :`DrawDebugType` "Persistent"))
  (if _returnvalue_2
    (bind (_bblockinghit _binitialoverlap _time _distance _location _impactpoint _normal _impactnormal _physmat _hitactor _hitcomponent) (`GameplayStatics.BreakHitResult` _outhit))
    (if (`SceneComponent.IsSimulatingPhysics` _hitcomponent "None")
      (if (< (`PrimitiveComponent.GetMass` _hitcomponent) 400.0)
        ;;[1 1 1] without component it makes it a push
        (`PhysicsHandleComponent.GrabComponentAtLocation` (`self.PhysicsHandle`) _hitcomponent "None" (`SceneComponent.K2_GetComponentLocation` _hitcomponent))
        (set `self.isholdingobject` true)
        (`KismetSystemLibrary.PrintString` "HOLDING IS TRUE"))
      (else
        (`KismetSystemLibrary.PrintString` "PHYSICS FAIL!!!")))))

(event `Drop`
  ;[1 1 1] Pick
  (`KismetSystemLibrary.PrintString` "Drop")
  (`PhysicsHandleComponent.ReleaseComponent` (`self.PhysicsHandle`))
  (set `self.isholdingobject` false)
  (`KismetSystemLibrary.PrintString` "HOLDING IS FALSE")
  (`PrimitiveComponent.AddImpulse` (`.HitComponent` (`GameplayStatics.BreakHitResult` (stale `Pickup` _outhit))) (* (`SceneComponent.GetForwardVector` (`self.forward_vector`)) (400.0 0.0 0.0)) "None" true)
  (`KismetSystemLibrary.PrintString` "THROW!"))

(event `self.ReceiveTick`
  (params (DeltaSeconds :type "Float (single-precision)"))
  ;[1 1 1] Pick
  (`PhysicsHandleComponent.SetTargetLocation` (`self.PhysicsHandle`) (`SceneComponent.K2_GetComponentLocation` (`self.HeldObjectLocation`))))

(event `EnhancedInput|/Game/Blueprints/IA_Pickup`
  (params (ActionValue :type "Float (double-precision)") (ElapsedSeconds :type "Float (double-precision)") (TriggeredSeconds :type "Float (double-precision)") (InputAction :type "InputAction Object Reference" :default "/Game/Blueprints/IA_Pickup.IA_Pickup"))
  ;[1 1 1] Pick
  (:`Started`
    (if (`self.isholdingobject`)
      (`self.Drop`)
      (`KismetSystemLibrary.PrintString` "Drop")
      (else
        (`self.Pickup`)
        (`KismetSystemLibrary.PrintString` "Pick up")))))

(fn `UserConstructionScript`)